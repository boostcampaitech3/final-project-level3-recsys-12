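; BP_BookShelf procedurally builds a horizontal row or vertical pile of books in its construction script.
; A loop randomly picks thin or thick book meshes, adding half of each scaled depth before and after placement, corrected for lean in rows.
; Parameters control disorder, scale, rotation and optional physics.
; Each book gets a dynamic cover material with random or chosen color and title texture, plus aging, dirt and roughness.
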(event EventBeginPlay)

(event Collision|EventActorBeginOverlap
  (params (OtherActor :type Actor%20Object%20Reference)))

(event EventTick
  (params (DeltaSeconds :type Float%20%28single-precision%29)))

(fn ConstructionScript
  (bind _position_disorder (Variables|Books|GetPosition%20disorder))
  (bind _random_scale (Variables|Books|GetRandom%20Scale))
  (bind _book_height (Variables|Books|GetBook%20Height))
  (bind _random_rotation (Variables|VerticalPile|GetRandom%20Rotation))
  (bind _random_scale_2 (Variables|Books|GetRandom%20Scale))
  (bind _position_disorder_2 (Variables|Books|GetPosition%20disorder))
  (bind _vertical_pile (Variables|Books|GetVertical%20Pile))
  (bind _returnvalue (not _vertical_pile))
  (bind _returnvalue_2 (* _random_scale 0.5))
  (bind _returnvalue_3 (* _random_scale_2 0.9))
  (bind _returnvalue_4 (* _position_disorder -1.0))
  (bind _returnvalue_5 (Math|Conversions|ToFloat(Boolean) _returnvalue))
  (bind _returnvalue_6 (- 1.0 _returnvalue_2))
  (bind _returnvalue_7 (+ 1.0 _returnvalue_2))
  (bind _returnvalue_8 (Math|Random|RandomFloatinRange _returnvalue_6 _returnvalue_7))
  (bind _returnvalue_9 (* _book_height _returnvalue_8))
  ;[1 0.2914 0.3113] Loop and Book type selection
  (for _index (range 0 (- (Variables|Books|GetNumber%20of%20Books) 1))
    (Variables|Default|SetCurrent%20is%20BookB (< (Math|Random|RandomFloatinRange 0.0 1e+02) (Variables|Books|Get%25%20of%20BookB%20%28Thin%29)))
    ;[1 1 1] Current Random Scale (Depth)
    (Variables|Default|SetCurrent%20RandomScale (* (Math|Random|RandomFloatinRange (- 1.0 _returnvalue_3) (+ 1.0 _returnvalue_3)) (Variables|Books|GetBook%20Depth)))
    (Utilities|FlowControl|Sequence
      (:then_0
        ;[1 1 1] Set Current Position
        (Variables|Default|SetCurrent%20Position (+ (Variables|Default|GetCurrent%20Position) (/ (* (select (Variables|Default|GetCurrent%20is%20BookB) (Math|Float|MakeLiteralFloat 1.0) (Math|Float|MakeLiteralFloat 5.5)) 0.5 (Variables|Default|GetCurrent%20RandomScale)) (Math|Trig|Cos(Degrees) (* (Variables|HorizontalShelf|GetLean) _returnvalue_5))))))
      (:then_1
        ;[1 1 1] Add Book Static Mesh
        (if (Variables|Default|GetCurrent%20is%20BookB)
          (bind _returnvalue_10 (AddComponent|AddStaticMeshComponent false (select (Variables|Books|GetVertical%20Pile) (Math|Transform|MakeTransform (Math|Vector|MakeVector (Math|Random|RandomFloatinRange _returnvalue_4 _position_disorder) (Math|Random|RandomFloatinRange _returnvalue_4 _position_disorder) (Variables|Default|GetCurrent%20Position)) (Math|Rotator|MakeRotator (select (Variables|VerticalPile|GetFlip%20Books) -9e+01 9e+01) 0.0 (Math|Random|RandomFloatinRange (* _random_rotation -1.0) _random_rotation)) (Math|Vector|MakeVector (* (Variables|Books|GetBook%20Width) (Math|Random|RandomFloatinRange _returnvalue_6 _returnvalue_7)) (Variables|Default|GetCurrent%20RandomScale) _returnvalue_9)) (Math|Transform|MakeTransform (Math|Vector|MakeVector (Variables|Default|GetCurrent%20Position) (Math|Random|RandomFloatinRange (* _position_disorder_2 -1.0) _position_disorder_2) 0.0) (Math|Rotator|MakeRotator (+ (Variables|HorizontalShelf|GetLean) (* (Math|Random|RandomFloatinRange -1.0 1.0) (Variables|HorizontalShelf|GetRandom%20Lean))) 0.0 -9e+01) (Math|Vector|MakeVector (* (Variables|Books|GetBook%20Width) (Math|Random|RandomFloatinRange _returnvalue_6 _returnvalue_7)) (Variables|Default|GetCurrent%20RandomScale) _returnvalue_9)))))
          (Variables|Default|SetCurrent%20Book%20Mesh _returnvalue_10)
          (else
            (bind _returnvalue_11 (AddComponent|AddStaticMeshComponent false (select (Variables|Books|GetVertical%20Pile) (Math|Transform|MakeTransform (Math|Vector|MakeVector (Math|Random|RandomFloatinRange _returnvalue_4 _position_disorder) (Math|Random|RandomFloatinRange _returnvalue_4 _position_disorder) (Variables|Default|GetCurrent%20Position)) (Math|Rotator|MakeRotator (select (Variables|VerticalPile|GetFlip%20Books) -9e+01 9e+01) 0.0 (Math|Random|RandomFloatinRange (* _random_rotation -1.0) _random_rotation)) (Math|Vector|MakeVector (* (Variables|Books|GetBook%20Width) (Math|Random|RandomFloatinRange _returnvalue_6 _returnvalue_7)) (Variables|Default|GetCurrent%20RandomScale) _returnvalue_9)) (Math|Transform|MakeTransform (Math|Vector|MakeVector (Variables|Default|GetCurrent%20Position) (Math|Random|RandomFloatinRange (* _position_disorder_2 -1.0) _position_disorder_2) 0.0) (Math|Rotator|MakeRotator (+ (Variables|HorizontalShelf|GetLean) (* (Math|Random|RandomFloatinRange -1.0 1.0) (Variables|HorizontalShelf|GetRandom%20Lean))) 0.0 -9e+01) (Math|Vector|MakeVector (* (Variables|Books|GetBook%20Width) (Math|Random|RandomFloatinRange _returnvalue_6 _returnvalue_7)) (Variables|Default|GetCurrent%20RandomScale) _returnvalue_9)))))
            (Variables|Default|SetCurrent%20Book%20Mesh _returnvalue_11)))
        (Transformation|AddLocalOffset (Variables|Default|GetCurrent%20Book%20Mesh) (Math|Vector|MakeVector 0.0 0.0 (select (Variables|Books|GetVertical%20Pile) (* (select (Variables|Default|GetCurrent%20is%20BookB) (Math|Float|MakeLiteralFloat 26.5) (Math|Float|MakeLiteralFloat 24.6)) _returnvalue_9 -0.5) (* (* (select (Variables|Default|GetCurrent%20is%20BookB) (Math|Float|MakeLiteralFloat 1.0) (Math|Float|MakeLiteralFloat 5.5)) 0.5 (Variables|Default|GetCurrent%20RandomScale)) (Math|Trig|Tan(Degrees) (Math|Float|Absolute(Float) (Variables|HorizontalShelf|GetLean)))))) false false)
        (Physics|SetSimulatePhysics (Variables|Default|GetCurrent%20Book%20Mesh) (Variables|Books|GetSimulate%20Physics))
        ;[1 1 1] Book Material
        (bind _returnvalue_12 (Rendering|Material|CreateDynamicMaterialInstance (Variables|Default|GetCurrent%20Book%20Mesh) 0 "/Game/Assets/Library/Materials/Books/M_Book_Cover.M_Book_Cover" "None" :!class /Script/Engine.PrimitiveComponent))
        (Rendering|Material|SetVectorParameterValueonMaterials (Variables|Default|GetCurrent%20Book%20Mesh) "Color" (Math|Conversions|ToVector(LinearColor) (select (Variables|BookMaterial|GetRandom%20Color) (Class|KismetMathLibrary|HSVtoRGB (Math|Random|RandomFloatinRange 0.0 3.6e+02) (Math|Random|RandomFloat) (Math|Random|RandomFloat) 1.0) (Math|Conversions|ToLinearColor(Color) (Variables|BookMaterial|GetColor)))))
        (Rendering|Material|SetScalarParameterValueonMaterials (Variables|Default|GetCurrent%20Book%20Mesh) "Old" (+ (Variables|BookMaterial|GetOld) (Math|Random|RandomFloatinRange 0.3 0.3)))
        ;[1 1 1] Random Book Cover Image
        (if (Variables|Default|GetCurrent%20is%20BookB)
          (switch int (select (Variables|BookMaterial|GetRandom%20Texture) (Math|Random|RandomIntegerinRange 1 7) (Variables|BookMaterial|GetTexture#))
            (:Default
              (Variables|Default|SetTexture "/Game/Assets/Library/Textures/Books/Covers/T_BookB_02_TravelGuide.T_BookB_02_TravelGuide" :!label _label))
            (:0
              (Variables|Default|SetTexture "/Game/Assets/Library/Textures/Books/Covers/T_BookB_01_ColorStories.T_BookB_01_ColorStories" :!label _label_2))
            (:1
              (goto _label_2))
            (:2
              (goto _label))
            (:3
              (Variables|Default|SetTexture "/Game/Assets/Library/Textures/Books/Covers/T_BookB_03_LandIsBlue.T_BookB_03_LandIsBlue"))
            (:4
              (Variables|Default|SetTexture "/Game/Assets/Library/Textures/Books/Covers/T_BookB_04_OpenYourMind.T_BookB_04_OpenYourMind"))
            (:5
              (Variables|Default|SetTexture "/Game/Assets/Library/Textures/Books/Covers/T_BookB_05_CivilizationChains.T_BookB_05_CivilizationChains"))
            (:6
              (Variables|Default|SetTexture "/Game/Assets/Library/Textures/Books/Covers/T_BookB_06_Entrance.T_BookB_06_Entrance"))
            (:7
              (Variables|Default|SetTexture "/Game/Assets/Library/Textures/Books/Covers/T_BookB_07_MyOrnament.T_BookB_07_MyOrnament")))
          (else
            (switch int (select (Variables|BookMaterial|GetRandom%20Texture) (Math|Random|RandomIntegerinRange 1 10) (Variables|BookMaterial|GetTexture#))
              (:0
                (Variables|Default|SetTexture "/Game/Assets/Library/Textures/Books/Covers/T_BookA_01_Mathematics.T_BookA_01_Mathematics" :!label _label_3))
              (:1
                (goto _label_3))
              (:2
                (Variables|Default|SetTexture "/Game/Assets/Library/Textures/Books/Covers/T_BookA_02_Physics.T_BookA_02_Physics"))
              (:3
                (Variables|Default|SetTexture "/Game/Assets/Library/Textures/Books/Covers/T_BookA_03_Chemistry.T_BookA_03_Chemistry"))
              (:4
                (Variables|Default|SetTexture "/Game/Assets/Library/Textures/Books/Covers/T_BookA_04_Geology.T_BookA_04_Geology"))
              (:5
                (Variables|Default|SetTexture "/Game/Assets/Library/Textures/Books/Covers/T_BookA_05_Guitar.T_BookA_05_Guitar"))
              (:6
                (Variables|Default|SetTexture "/Game/Assets/Library/Textures/Books/Covers/T_BookA_06_Atlas.T_BookA_06_Atlas"))
              (:7
                (Variables|Default|SetTexture "/Game/Assets/Library/Textures/Books/Covers/T_BookA_07_Bible.T_BookA_07_Bible"))
              (:8
                (Variables|Default|SetTexture "/Game/Assets/Library/Textures/Books/Covers/T_BookA_08_Architecture.T_BookA_08_Architecture"))
              (:9
                (Variables|Default|SetTexture "/Game/Assets/Library/Textures/Books/Covers/T_BookA_09_GreenVelo.T_BookA_09_GreenVelo"))
              (:10
                (Variables|Default|SetTexture "/Game/Assets/Library/Textures/Books/Covers/T_BookA_10_DoNotDisturb.T_BookA_10_DoNotDisturb")))))
        (Rendering|Material|SetTextureParameterValue _returnvalue_12 "Texture" (Variables|Default|GetTexture))
        ;[1 1 1] Random Dirt UV Coord
        (Rendering|Material|SetScalarParameterValue _returnvalue_12 "DirtTexShiftU" (Math|Random|RandomFloat) :!class /Script/Engine.MaterialInstanceDynamic)
        (Rendering|Material|SetScalarParameterValue _returnvalue_12 "DirtTexShiftV" (Math|Random|RandomFloat) :!class /Script/Engine.MaterialInstanceDynamic)
        ;[1 1 1] Roughness and Dirt
        (Rendering|Material|SetScalarParameterValue _returnvalue_12 "Roughness" (Variables|BookMaterial|GetRoughness) :!class /Script/Engine.MaterialInstanceDynamic)
        (Rendering|Material|SetScalarParameterValue _returnvalue_12 "Dirt" (Variables|BookMaterial|GetDirt) :!class /Script/Engine.MaterialInstanceDynamic))
      (:then_2
        (Variables|Default|SetCurrent%20Position (+ (Variables|Default|GetCurrent%20Position) (/ (* (select (Variables|Default|GetCurrent%20is%20BookB) (Math|Float|MakeLiteralFloat 1.0) (Math|Float|MakeLiteralFloat 5.5)) 0.5 (Variables|Default|GetCurrent%20RandomScale)) (Math|Trig|Cos(Degrees) (* (Variables|HorizontalShelf|GetLean) _returnvalue_5))) (* (Variables|HorizontalShelf|GetSpacing) _returnvalue_5)))))))

(fn NewFunction0)